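; An example Blueprint that creates a ROS 2 node and publishes string messages in three different ways.
; On BeginPlay it initializes the node and registers a non-loop, a loop and a custom-class publisher.
; The non-loop publisher sends one message after a delay, while the loop publisher fills each message through a delegate that appends an incrementing count.
; The custom string publisher only has its Message property set before registration.
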(event `self.ReceiveBeginPlay`
  (bind _publisher (`ROS2PublisherComponent.Publisher` (`self.ROS2NonLoopPublisher`)))
  (bind _publisher_2 (`ROS2PublisherComponent.Publisher` (`self.ROS2LoopPublisher`)))
  (bind _publisher_3 (`ROS2CustomPublisherComponent.Publisher` (`self.ROS2CustomPublisher`)))
  ; Init Node
  (`ROS2NodeComponent.Init` (`self.ROS2Node`))
  (`|ExecutionSequence`
    (:`then_0`
      ; Non Loop Publisher
      (`ROS2NodeComponent.AddPublisher` (`self.ROS2Node`) _publisher)
      (`KismetSystemLibrary.Delay` 4.0)
      (`ROS2StrMsg.SetMsg` (cast `ROS2StrMsg` (`ROS2Topic.TopicMessage` _publisher) :!pure true) (make `ROSStr` "Hello From BP Non Loop Publisher  "))
      (`ROS2Publisher.Publish` (`ROS2PublisherComponent.Publisher` (`self.ROS2NonLoopPublisher`))))
    (:`then_1`
      ; Loop Publisher
      (`ROS2Publisher.SetDelegates` _publisher_2 (delegate `TimerEvent`))
      (`ROS2NodeComponent.AddPublisher` (`self.ROS2Node`) _publisher_2))
    (:`then_2`
      ; Custom Publisher Class
      (set `RRROS2StringPublisher.Message` "Hello From BP Loop Publisher  " (cast `RRROS2StringPublisher` _publisher_3 :!pure true))
      (`ROS2NodeComponent.AddPublisher` (`self.ROS2Node`) _publisher_3))))

(event `TimerEvent`
  (params (InTopicMessage :type "ROS2GenericMsg Object Reference"))
  (bind _count (`self.count`))
  ; Loop Publisher
  (`ROS2StrMsg.SetMsg` (cast `ROS2StrMsg` InTopicMessage :!pure true) (make `ROSStr` (`KismetStringLibrary.Concat_StrStr` "Hello From BP Loop Publisher  " (`KismetStringLibrary.Conv_IntToString` _count))))
  (`/Engine/EditorBlueprintResources/StandardMacros.IncrementInt` _count))

(fn `UserConstructionScript`)